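; BP_ColorBulb is a VR-hand-interactable bulb actor that cycles its sphere's material through a list of colors.
; A box trigger tracks whether a BP_HandController overlaps it.
; On a ChangeBulbColor interface color request, an active, overlapped bulb advances the color index with wraparound.
; SetNewMat, also triggered by material refresh requests, applies that color when active or a glass material when inactive.
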(event ChangeColorRequest(ChangeBulbColor)
  (if (Variables|Default|GetIsActivate)
    (if (Variables|Default|GetIs%20overlapping)
      (if (>= (+ (Variables|Default|GetTheColor) 1) (Utilities|Array|Length (Variables|Default|GetMaterials)))
        (Variables|Default|SetTheColor 0)
        (else
          (Variables|Default|SetTheColor (+ (Variables|Default|GetTheColor) 1))))
      (CallFunction|SetNewMat))))

(event ChangeMatRequest(ChangeBulbColor)
  (CallFunction|SetNewMat))

(event OnComponentBeginOverlap(Box)
  (params (OverlappedComponent :type Primitive%20Component%20Object%20Reference) (OtherActor :type Actor%20Object%20Reference) (OtherComp :type Primitive%20Component%20Object%20Reference) (OtherBodyIndex :type Integer) (bFromSweep :type Boolean) (SweepResult :type Hit%20Result%20Structure%20%28by%20ref%29))
  (if (== (Utilities|GetClass OtherActor) "/Game/Blueprints/BP_HandController.BP_HandController_C")
    (Variables|Default|SetIs%20overlapping true)))

(event OnComponentEndOverlap(Box)
  (params (OverlappedComponent :type Primitive%20Component%20Object%20Reference) (OtherActor :type Actor%20Object%20Reference) (OtherComp :type Primitive%20Component%20Object%20Reference) (OtherBodyIndex :type Integer))
  (if (== (Utilities|GetClass OtherActor) "/Game/Blueprints/BP_HandController.BP_HandController_C")
    (Variables|Default|SetIs%20overlapping false)))

(event EventBeginPlay)

(event Collision|EventActorBeginOverlap
  (params (OtherActor :type Actor%20Object%20Reference)))

(event EventTick
  (params (DeltaSeconds :type Float%20%28single-precision%29)))

(fn ConstructionScript)

(fn SetNewMat
  (bind _sphere (Variables|Default|GetSphere))
  (if (Variables|Default|GetIsActivate)
    (Rendering|Material|SetMaterial _sphere 0 (Utilities|Array|Get(acopy) (Variables|Default|GetMaterials) (Variables|Default|GetTheColor)))
    (else
      (Rendering|Material|SetMaterial _sphere 0 "/DatasmithContent/Materials/FBXImporter/VRED/Glass.Glass"))))