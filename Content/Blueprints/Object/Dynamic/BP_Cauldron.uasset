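; BP_Cauldron is a puzzle cauldron that rewards a power bar once every recipe ingredient is inside its box.
; Overlap begin and end events set each grabbable ingredient's flag in IngredientIn by matching its actor against the Recette array.
; When all flags are true, it marks the game instance's second PuzzleCompleted entry, then after a short delay destroys the ingredients and spawns BP_PowerBar at the box.
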(event OnComponentBeginOverlap(Box)
  (params (OverlappedComponent :type Primitive%20Component%20Object%20Reference) (OtherActor :type Actor%20Object%20Reference) (OtherComp :type Primitive%20Component%20Object%20Reference) (OtherBodyIndex :type Integer) (bFromSweep :type Boolean) (SweepResult :type Hit%20Result%20Structure%20%28by%20ref%29))
  (bind _returnvalue (Actor|GetComponentbyClass OtherActor "/Script/VR_Portalventure.IsGrabbable"))
  (Utilities|IsValid _returnvalue
    (:Is%20Valid
      (for (_array_element _array_index) (Variables|Default|GetRecette)
        (if (== (Components|GetOwner _returnvalue) _array_element)
          (Utilities|Array|SetArrayElem (Variables|Default|GetIngredientIn) _array_index (== (Components|GetOwner _returnvalue) _array_element))))
      (if (Utilities|Array|ContainsItem (Variables|Default|GetIngredientIn) false)
        (Development|PrintString "Not enough")
        (else
          (Development|PrintString "Destroy elements")
          (bind _asbp_game_instance (Utilities|Casting|CastToBP_GameInstance (Game|GetGameInstance)))
          (Utilities|Array|SetArrayElem (Variables|/Game/Blueprints/GameInstance/BP_GameInstance.BP_GameInstance_C|GetPuzzleCompleted _asbp_game_instance) 1 true)
          (Utilities|FlowControl|Delay 1.0)
          (for _array_element_2 (Variables|Default|GetRecette)
            (Actor|DestroyActor _array_element_2))
          (Game|SpawnActorfromClass "/Game/Blueprints/Object/Static/BP_PowerBar.BP_PowerBar_C" (Math|Transform|MakeTransform (Transformation|GetWorldLocation (Variables|Default|GetBox)) "0, 0, 0" "1,1,1") "AdjustIfPossibleButAlwaysSpawn" 0 0))))))

(event OnComponentEndOverlap(Box)
  (params (OverlappedComponent :type Primitive%20Component%20Object%20Reference) (OtherActor :type Actor%20Object%20Reference) (OtherComp :type Primitive%20Component%20Object%20Reference) (OtherBodyIndex :type Integer))
  (bind _returnvalue (Actor|GetComponentbyClass OtherActor "/Script/VR_Portalventure.IsGrabbable"))
  (Utilities|IsValid _returnvalue
    (:Is%20Valid
      (for (_array_element _array_index) (Variables|Default|GetRecette)
        (if (== (Components|GetOwner _returnvalue) _array_element)
          (Utilities|Array|SetArrayElem (Variables|Default|GetIngredientIn) _array_index (not (== (Components|GetOwner _returnvalue) _array_element))))))))

(event EventBeginPlay)

(event Collision|EventActorBeginOverlap
  (params (OtherActor :type Actor%20Object%20Reference)))

(event EventTick
  (params (DeltaSeconds :type Float%20%28single-precision%29)))

(fn ConstructionScript)