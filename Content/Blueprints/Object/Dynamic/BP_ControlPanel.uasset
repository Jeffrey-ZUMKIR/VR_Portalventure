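; BP_ControlPanel is a panel actor that becomes active when a BP_PowerBar is placed in its trigger box.
; On overlap it snaps the bar to its Scene component, turns off the bar's physics, fixes its rotation and notifies it through Attached.
; It then sets Active and passes that state to PanelActivate.
; When the bar leaves the box, Active is cleared and PanelActivate is called again.
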(event OnComponentBeginOverlap(Box)
  (params (OverlappedComponent :type Primitive%20Component%20Object%20Reference) (OtherActor :type Actor%20Object%20Reference) (OtherComp :type Primitive%20Component%20Object%20Reference) (OtherBodyIndex :type Integer) (bFromSweep :type Boolean) (SweepResult :type Hit%20Result%20Structure%20%28by%20ref%29))
  (if (== (Utilities|GetClass OtherActor) "/Game/Blueprints/Object/Static/BP_PowerBar.BP_PowerBar_C")
    (bind _asbp_power_bar (Utilities|Casting|CastToBP_PowerBar OtherActor))
    (Transformation|AttachComponentToComponent OtherActor (Variables|Default|GetScene) "None" "SnapToTarget" "SnapToTarget" "KeepWorld" true)
    (Physics|SetSimulatePhysics (Variables|/Game/Blueprints/Object/Static/BP_PowerBar.BP_PowerBar_C|GetBar _asbp_power_bar) false)
    (Transformation|SetWorldRotation (Variables|/Game/Blueprints/Object/Static/BP_PowerBar.BP_PowerBar_C|GetBar _asbp_power_bar) "-90.000000, 0, 0" false false)
    (Default|Attached _asbp_power_bar)
    (bind _output_get (Variables|Default|SetActive true))
    (Class|ControlPanel|PanelActivate _output_get)))

(event OnComponentEndOverlap(Box)
  (params (OverlappedComponent :type Primitive%20Component%20Object%20Reference) (OtherActor :type Actor%20Object%20Reference) (OtherComp :type Primitive%20Component%20Object%20Reference) (OtherBodyIndex :type Integer))
  (if (== (Utilities|GetClass OtherActor) "/Game/Blueprints/Object/Static/BP_PowerBar.BP_PowerBar_C")
    (bind _output_get (Variables|Default|SetActive false))
    (Class|ControlPanel|PanelActivate _output_get)))

(event EventBeginPlay)

(event Collision|EventActorBeginOverlap
  (params (OtherActor :type Actor%20Object%20Reference)))

(event EventTick
  (params (DeltaSeconds :type Float%20%28single-precision%29)))

(fn ConstructionScript)